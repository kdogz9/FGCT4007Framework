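; BP_Money2 is a shootable money stack that awards score to the player when hit.
; Each BPIShoot interface call adds one to the first-person character's Score and to the stack's own LocalScore counter.
; Once LocalScore reaches 100, further shots award nothing and swap the static mesh to a wet money material.
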(event `self.BPI_Shoot`
  (bind _localscore (`self.LocalScore`))
  ;[1 0.03646 0.8556] Increases score by 1 when called
  (bind _asbp_first_person_character (cast `/Game/Dynamic/Blueprints/Core/MC/BP_FirstPersonCharacter` (`GameplayStatics.GetPlayerCharacter` 0)))
  (if (== _localscore 100)
    ;;[1 1 1] changes to wet when hit 100
    (`PrimitiveComponent.SetMaterial` (`self.StaticMesh`) 0 "/Game/Assets/MoneyStackTexWet_Mat.MoneyStackTexWet_Mat")
    (else
      (set `/Game/Dynamic/Blueprints/Core/MC/BP_FirstPersonCharacter.Score` (+ (`/Game/Dynamic/Blueprints/Core/MC/BP_FirstPersonCharacter.Score` _asbp_first_person_character) 1) _asbp_first_person_character)
      (set `self.LocalScore` (+ _localscore 1)))))

(fn `UserConstructionScript`)