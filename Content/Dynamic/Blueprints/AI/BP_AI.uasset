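; BP_AI is an enemy pawn that roams randomly, chases pawns it sees, and shows the end screen when its Box overlaps the player.
; Roaming repeats after each successful AIMoveTo to a random reachable point.
; PawnSensing redirects movement to the seen pawn, with a retriggerable delay resuming roaming once sightings stop.
; A water projectile overlap kills it, ragdolling the mesh before destroying the actor.
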(event `self.ReceiveBeginPlay`
  ;[1 1 1] Makes the AI roam around
  (`self.Random Roam`))

(event `Kill`
  ;[1 1 1] Kills AI when shot
  (`PrimitiveComponent.SetCollisionEnabled` (`self.Mesh`) "PhysicsOnly")
  (`PrimitiveComponent.SetSimulatePhysics` (`self.Mesh`) true)
  (`KismetSystemLibrary.Delay` 3.0)
  (`self.K2_DestroyActor`))

(event `Random Roam`
  ;[1 1 1] Makes the AI roam around
  (`|AIMoveTo` self (`NavigationSystemV1.K2_GetRandomReachablePointInRadius` (`self.K2_GetActorLocation`) 2500.0 null null) null
    (:`OnSuccess`
      ;;[1 1 1] Starts again after success
      (`self.Random Roam`))))

(event `self.PawnSensing.OnSeePawn`
  (params (Pawn :type "Pawn Object Reference"))
  ;[1 1 1] Once AI sees a pawn it will move towards them
  (`|ExecutionSequence`
    (:`then_0`
      (`|AIMoveTo` self (0.0 0.0 0.0) Pawn))
    (:`then_1`
      ;;[1 1 1] Restarts the AI seeing the pawn so that its not constantly chasing us
      (`KismetSystemLibrary.RetriggerableDelay` 1.0)
      (`self.Random Roam`))))

(event `self.Box.OnComponentBeginOverlap`
  (params (OverlappedComponent :type "PrimitiveComponent Object Reference") (OtherActor :type "Actor Object Reference") (OtherComp :type "PrimitiveComponent Object Reference") (OtherBodyIndex :type Integer) (bFromSweep :type Boolean) (SweepResult :type "HitResult Structure (by ref)"))
  ;[1 1 1] End screen when hit
  (cast `/Game/Dynamic/Blueprints/Core/MC/BP_FirstPersonCharacter` OtherActor
    (:`then`
      (bind _returnvalue (`|CreateWidget` "/Game/Dynamic/Blueprints/UI/WBP_EndScreen.WBP_EndScreen_C"))
      (`UserWidget.AddToViewport` _returnvalue 0)
      (`WidgetBlueprintLibrary.SetInputMode_GameOnly` (`GameplayStatics.GetPlayerController` 0)))
    (:`CastFailed`
      ;;[1 1 1] kills AI
      (cast `/Game/Dynamic/Blueprints/Shooting/BP_WaterProjectile` OtherActor)
      (`self.Kill`))))

(fn `GetGameplayTags`
  (returns (OwnedGameplayTags :type "GameplayTagContainer Structure"))
  (return (`self.OwnedGameplayTags`)))

(fn `UserConstructionScript`)