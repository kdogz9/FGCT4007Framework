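; Manager actor that spawns BP_AI characters at the BPSpawnLocations actor's position.
; On BeginPlay it registers itself as BPAiSpawnManager on the GM_4007 game mode.
; When SpawnAI is called and fewer than AmountOfAI BP_AI actors exist, it loops over AmountOfAI to spawn a whole batch rather than topping up the shortfall.
; Spawns adjust for collision or are skipped, and each iteration prints a debug string.
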(event `SpawnAI`
  (bind _outactors (`GameplayStatics.GetAllActorsOfClass` "/Game/Dynamic/Blueprints/AI/BP_AI.BP_AI_C"))
  (if (< (`KismetArrayLibrary.Array_Length` _outactors) (`self.AmountOfAI`))
    (for _ (range (+ (`self.AmountOfAI`) 1))
      (`|SpawnActorFromClass` "/Game/Dynamic/Blueprints/AI/BP_AI.BP_AI_C" (`KismetMathLibrary.Conv_VectorToTransform` (`self.K2_GetActorLocation` (`self.BP_SpawnLocations`))) "AdjustIfPossibleButDontSpawnIfColliding" "MultiplyWithRoot" null null)
      (`KismetSystemLibrary.PrintString` "Hello"))))

(event `self.ReceiveBeginPlay`
  (bind _asgm_4007 (cast `/Game/Dynamic/Blueprints/Core/GM_4007` (`GameplayStatics.GetGameMode`)))
  (set `/Game/Dynamic/Blueprints/Core/GM_4007.BP_AiSpawnManager` self _asgm_4007))

(fn `UserConstructionScript`)