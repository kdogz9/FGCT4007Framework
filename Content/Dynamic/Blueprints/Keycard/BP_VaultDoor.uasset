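; BP_VaultDoor is an interactable vault door that swings open only when the player carries the vault keycard.
; BeginPlay caches the first-person character, and Interact checks that character's VaultKeycard flag.
; A FlipFlop alternately plays and reverses a Timeline that lerps the door mesh's yaw, so repeated interactions open and close it.
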(event `self.ReceiveBeginPlay`
  ;[1 1 1] For key card system , just casting to the player
  (bind _asbp_first_person_character (cast `/Game/Dynamic/Blueprints/Core/MC/BP_FirstPersonCharacter` (`GameplayStatics.GetPlayerCharacter` 0)))
  (set `self.As BP First Person Character` _asbp_first_person_character))

(event `/Game/Dynamic/Blueprints/Core/Interfaces/BPI_Interact.Interact`
  ;[1 1 1] Opens door when keycard is in the player inventory
  (if (`.VaultKeycard_1_69E8444D4790CC2EC974AABD976321E7` (break `/Game/Dynamic/Blueprints/Keycard/BPS-Keycards` (`/Game/Dynamic/Blueprints/Core/MC/BP_FirstPersonCharacter.VaultKeycard` (`self.As BP First Person Character`))))
    (`/Engine/EditorBlueprintResources/StandardMacros.FlipFlop`
      (:`A`
        (bind (_direction _newtrack_0) (`Timeline|Timeline` :!label _label)
          (:`Update`
            (`SceneComponent.K2_SetRelativeRotation` (`self.VaultDoor`) (`KismetMathLibrary.MakeRotator` 0.0 0.0 (`KismetMathLibrary.Lerp` 0.0 -100.0 _newtrack_0)) false false))))
      (:`B`
        (goto _label :!via `Reverse`)))))

(fn `UserConstructionScript`)