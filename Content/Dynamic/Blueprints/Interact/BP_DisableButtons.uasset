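; BP_DisableButtons is an interactable that disables CCTV screens and buys the player extra time before the police arrive.
; On Interact, a DoOnce gate lets it fire once, adding seconds to the timer on the first-person character.
; It then loops over a range of material slots on the CameraScreen's screen mesh, setting glossy black to simulate powered-off monitors, with a leftover debug print per slot.
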(event `/Game/Dynamic/Blueprints/Core/Interfaces/BPI_Interact.Interact`
  (`/Engine/EditorBlueprintResources/StandardMacros.DoOnce` false
    (:`Completed`
      ;[1 1 1] Adds extra time onto the timer , delaying police arrival
      (bind _asbp_first_person_character (cast `/Game/Dynamic/Blueprints/Core/MC/BP_FirstPersonCharacter` (`GameplayStatics.GetPlayerCharacter` 0)))
      (bind _timer (`/Game/Dynamic/Blueprints/Core/MC/BP_FirstPersonCharacter.Timer` _asbp_first_person_character))
      (set `/Game/Dynamic/Blueprints/UI/WBP_Timer.Seconds` (+ (`/Game/Dynamic/Blueprints/UI/WBP_Timer.Seconds` _timer) 10.0) _timer)
      ;[1 1 1] Then changes the material of the screens to black to simulate them being off
      (for _index (range 2 18)
        (`PrimitiveComponent.SetMaterial` (`/Game/Dynamic/Blueprints/CCTV/BP_CameraScreen.Screen` (`self.CameraScreen`)) _index "/Game/Dynamic/AssetsvilleTown/Materials/MI_glossyBlack.MI_glossyBlack")
        (`KismetSystemLibrary.PrintString` "Hello")))))

(fn `UserConstructionScript`)