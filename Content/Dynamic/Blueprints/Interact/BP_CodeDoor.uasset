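; BP_CodeDoor is an interactable door that uses a keypad widget for code entry.
; The box trigger enables input and shows a text prompt while the first-person character is inside.
; Interact toggles WBP_CodeSyetm, cursor and input mode through a FlipFlop, and leaving the box also removes the widget without resetting the FlipFlop.
; DoorOpenCode, not called within this graph, plays a timeline that swings the door open on yaw.
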(event `DoorOpenCode`
  ;[1 0.007891 0.8932] Code system
  ;;[1 1 1] Opens door using code system
  (bind (_direction _doordegree) (`Timeline|Timeline`)
    (:`Update`
      (`SceneComponent.K2_SetRelativeRotation` (`self.Door`) (`KismetMathLibrary.MakeRotator` 0.0 0.0 (`KismetMathLibrary.Lerp` 0.0 90.0 _doordegree)) false false))))

(event `/Game/Dynamic/Blueprints/Core/Interfaces/BPI_Interact.Interact`
  (bind _returnvalue (`GameplayStatics.GetPlayerController` 0))
  ;[1 0.007891 0.8932] Code system
  ;;[1 1 1] shows key pad when E is pressed
  (`/Engine/EditorBlueprintResources/StandardMacros.FlipFlop`
    (:`A`
      (bind _returnvalue_2 (`|CreateWidget` "/Game/Dynamic/Blueprints/UI/WBP_CodeSyetm.WBP_CodeSyetm_C"))
      (set `self.CodeWidget` _returnvalue_2)
      (`UserWidget.AddToViewport` _returnvalue_2 0)
      (`WidgetBlueprintLibrary.SetInputMode_GameAndUIEx` _returnvalue _returnvalue_2)
      (set `PlayerController.bShowMouseCursor` true _returnvalue))
    (:`B`
      ;;[1 1 1] Another way to remove the keypad is if the player hits E again
      (`Widget.RemoveFromParent` (`self.CodeWidget`) :!label _label)
      (`WidgetBlueprintLibrary.SetInputMode_GameOnly` _returnvalue)
      (set `PlayerController.bShowMouseCursor` false _returnvalue))))

(event `self.Box.OnComponentBeginOverlap`
  (params (OverlappedComponent :type "PrimitiveComponent Object Reference") (OtherActor :type "Actor Object Reference") (OtherComp :type "PrimitiveComponent Object Reference") (OtherBodyIndex :type Integer) (bFromSweep :type Boolean) (SweepResult :type "HitResult Structure (by ref)"))
  ;[1 0.007891 0.8932] Code system
  ;;[1 1 1] when stepped outside of collision box the widget is removed
  (cast `/Game/Dynamic/Blueprints/Core/MC/BP_FirstPersonCharacter` OtherActor)
  (`self.EnableInput` (`GameplayStatics.GetPlayerController` 0))
  (`SceneComponent.SetVisibility` (`self.TextRender`) true false))

(event `self.Box.OnComponentEndOverlap`
  (params (OverlappedComponent :type "PrimitiveComponent Object Reference") (OtherActor :type "Actor Object Reference") (OtherComp :type "PrimitiveComponent Object Reference") (OtherBodyIndex :type Integer))
  ;[1 0.007891 0.8932] Code system
  ;;[1 1 1] when stepped outside of collision box the widget is removed
  (cast `/Game/Dynamic/Blueprints/Core/MC/BP_FirstPersonCharacter` OtherActor)
  (`self.DisableInput` (`GameplayStatics.GetPlayerController` 0))
  (`SceneComponent.SetVisibility` (`self.TextRender`) false false)
  ;;[1 1 1] Another way to remove the keypad is if the player hits E again
  (`/Engine/EditorBlueprintResources/StandardMacros.IsValid` (`self.CodeWidget`)
    (:`Is Valid`
      (goto _label))))

(fn `UserConstructionScript`)